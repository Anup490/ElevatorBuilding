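; Elevator actor that carries BP_Player upward, with a WBP_Lift widget as its interface.
; Overlapping the trigger box stores the player and shows the widget and mouse cursor; leaving hides both.
; OnGo closes the door, instantly offsets lift and player box up one fixed step, then reopens after a delay, toggling player inside/outside state.
; The Floor argument is unused, and an up/down oscillation branch using MoveDown never runs.
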(event `self.ReceiveBeginPlay`
  (`self.OpenDoor`)
  (bind _returnvalue (`|CreateWidget` "/Game/CollaborativeViewer/ElevatorBuilding/WBP_Lift.WBP_Lift_C"))
  (bind _output_get (set `self.HUD` _returnvalue))
  (`/Game/CollaborativeViewer/ElevatorBuilding/WBP_Lift.SetLift` _output_get self))

(event `self.ReceiveTick`
  (params (DeltaSeconds :type "Float (single-precision)")))

(event `self.Box.OnComponentBeginOverlap`
  (params (OverlappedComponent :type "PrimitiveComponent Object Reference") (OtherActor :type "Actor Object Reference") (OtherComp :type "PrimitiveComponent Object Reference") (OtherBodyIndex :type Integer) (bFromSweep :type Boolean) (SweepResult :type "HitResult Structure (by ref)"))
  (bind _hud (`self.HUD`))
  (bind _asbp_player (cast `/Game/CollaborativeViewer/ElevatorBuilding/BP_Player` OtherActor))
  (set `self.Player` _asbp_player)
  (if (not (`Widget.IsInViewport` _hud))
    (`UserWidget.AddToViewport` _hud 0))
  (set `PlayerController.bShowMouseCursor` true (`GameplayStatics.GetPlayerController` 0)))

(event `self.Box.OnComponentEndOverlap`
  (params (OverlappedComponent :type "PrimitiveComponent Object Reference") (OtherActor :type "Actor Object Reference") (OtherComp :type "PrimitiveComponent Object Reference") (OtherBodyIndex :type Integer))
  (`Widget.RemoveFromParent` (`self.HUD`))
  (set `PlayerController.bShowMouseCursor` false (`GameplayStatics.GetPlayerController` 0)))

(event `On Go`
  (params (Floor :type Integer))
  (bind _returnvalue (`GameplayStatics.GetPlayerController` 0))
  (bind _player (`self.Player`))
  (bind _hud (`self.HUD`))
  (`self.CloseDoor`)
  (`/Game/CollaborativeViewer/ElevatorBuilding/BP_Player.Inside Lift` _player)
  (`self.MoveUp`)
  (`Widget.RemoveFromParent` (`self.HUD`))
  (set `PlayerController.bShowMouseCursor` false _returnvalue)
  (`KismetSystemLibrary.Delay` 1.0)
  (`/Game/CollaborativeViewer/ElevatorBuilding/BP_Player.Outside Lift` _player)
  (if (not (`Widget.IsInViewport` _hud))
    (`UserWidget.AddToViewport` _hud 0))
  (`self.OpenDoor`)
  (set `PlayerController.bShowMouseCursor` true _returnvalue))

(fn `CloseDoor`
  (`SceneComponent.K2_AddWorldOffset` (`self.Door`) (-200.0 0.0 0.0) false false))

(fn `MoveDown`
  (`SceneComponent.K2_AddWorldOffset` (`self.DefaultSceneRoot`) (0.0 0.0 -5.0) false false))

(fn `MoveUp`
  (`SceneComponent.K2_AddWorldOffset` (`self.DefaultSceneRoot`) (0.0 0.0 200.0) false false)
  (`SceneComponent.K2_AddWorldOffset` (`/Game/CollaborativeViewer/ElevatorBuilding/BP_Player.Box` (`self.Player`)) (0.0 0.0 200.0) false false))

(fn `OpenDoor`
  (`SceneComponent.K2_AddWorldOffset` (`self.Door`) (200.0 0.0 0.0) false false))

(fn `UserConstructionScript`)