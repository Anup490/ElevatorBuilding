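; GM_Main, by name a game mode, builds the elevator building's stack of floors and basements at runtime from requested counts.
; SpawnFloors stacks BP_Floor actors upward and SpawnBasements stacks BP_Basement actors downward at fixed spacing, numbering basements negatively.
; Each first calls its Clear function, which destroys the previous actors by stored counter and resets the spawn transform, without emptying the array.
; Event graph and construction script are empty.
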(event `self.ReceiveBeginPlay`)

(fn `ClearBasements`
  (for _index (range 1 (+ (`self.BasementCounter`) 1))
    (`self.K2_DestroyActor` (`|GetArrayItem` (`self.Basements`) (- _index 1)))
    (set `self.BasementLoc` (`KismetMathLibrary.MakeTransform` (-688.0 -400.0 -400.0)))))

(fn `ClearFloors`
  (for _index (range 1 (+ (`self.FloorCounter`) 1))
    (`self.K2_DestroyActor` (`|GetArrayItem` (`self.Floors`) (- _index 1)))
    (set `self.Loc` (`KismetMathLibrary.MakeTransform` (-688.0 -400.0 80.0)))))

(fn `SpawnBasements`
  (params (Count :type Integer))
  (bind _basementloc_location (`KismetMathLibrary.BreakTransform` (`self.BasementLoc`)))
  (`self.ClearBasements`)
  (bind _output_get (set `self.BasementCounter` Count))
  (for _index (range 1 (+ _output_get 1))
    (bind _returnvalue (`|SpawnActorFromClass` "/Game/CollaborativeViewer/ElevatorBuilding/BP_Basement.BP_Basement_C" (`self.BasementLoc`) "Undefined" "OverrideRootScale" null null))
    (`KismetArrayLibrary.Array_Insert` (`self.Basements`) _returnvalue (- _index 1))
    (`/Game/CollaborativeViewer/ElevatorBuilding/BP_Basement.Set Floor Name` _returnvalue (* _index -1))
    (set `self.BasementLoc` (`KismetMathLibrary.MakeTransform` (- _basementloc_location (0.0 0.0 200.0))))))

(fn `SpawnFloors`
  (params (Count :type Integer))
  (bind _loc_location (`KismetMathLibrary.BreakTransform` (`self.Loc`)))
  (`self.ClearFloors`)
  (bind _output_get (set `self.FloorCounter` Count))
  (for _index (range 1 (+ _output_get 1))
    (bind _returnvalue (`|SpawnActorFromClass` "/Game/CollaborativeViewer/ElevatorBuilding/BP_Floor.BP_Floor_C" (`self.Loc`) "Undefined" "OverrideRootScale" null null))
    (`KismetArrayLibrary.Array_Insert` (`self.Floors`) _returnvalue (- _index 1))
    (`/Game/CollaborativeViewer/ElevatorBuilding/BP_Floor.Set Floor Name` _returnvalue _index)
    (set `self.Loc` (`KismetMathLibrary.MakeTransform` (+ _loc_location (0.0 0.0 200.0))))))

(fn `UserConstructionScript`)