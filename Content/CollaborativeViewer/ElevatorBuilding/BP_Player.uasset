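; BP_Player is a player-controlled actor in the CollaborativeViewer ElevatorBuilding folder that handles basic walking and horizontal looking.
; WalkForward and WalkRight axes offset the actor along player controller 0's forward and right vectors at a fixed step per call.
; Movement is neither swept for collision nor scaled by delta time.
; LookRight adds controller yaw, while BeginPlay, Tick, overlap and the construction script are empty.
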(event `self.ReceiveBeginPlay`)

(event `InputAxis|WalkForward`
  (params (AxisValue :type "Float (single-precision)"))
  (`self.K2_AddActorWorldOffset` (* (`self.GetActorForwardVector` (`GameplayStatics.GetPlayerController` 0)) (* AxisValue 5.0))))

(event `InputAxis|WalkRight`
  (params (AxisValue :type "Float (single-precision)"))
  (`self.K2_AddActorWorldOffset` (* (`self.GetActorRightVector` (`GameplayStatics.GetPlayerController` 0)) (* AxisValue 5.0))))

(event `InputAxis|LookRight`
  (params (AxisValue :type "Float (single-precision)"))
  (`self.AddControllerYawInput` AxisValue))

(fn `UserConstructionScript`)